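; BP_Banana is a spinning pickup that grants the player an extra life.
; Tick yaws the actor at RotationSpeed, scaled by delta time.
; When SM_Banana begins an overlap, the banana destroys itself before the BP_Player cast, so any overlapping actor consumes it.
; If that actor is a BP_Player, it increments LivesCount and refreshes the player's health widget.
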(event OnComponentBeginOverlap(SM_Banana)
  (params (OverlappedComponent :type Primitive%20Component%20Object%20Reference) (OtherActor :type Actor%20Object%20Reference) (OtherComp :type Primitive%20Component%20Object%20Reference) (OtherBodyIndex :type Integer) (bFromSweep :type Boolean) (SweepResult :type Hit%20Result%20Structure%20%28by%20ref%29))
  (Actor|DestroyActor)
  (bind _asbp_player (Utilities|Casting|CastToBP_Player OtherActor))
  (Math|Integer|IncrementInt (Variables|/Game/InfiniteMatrix/Blueprints/BP_Player.BP_Player_C|GetLivesCount _asbp_player)
    (:%20%20
      (Variables|/Game/InfiniteMatrix/UI/HealthWidget.HealthWidget_C|SetLivesInfo (Variables|/Game/InfiniteMatrix/Blueprints/BP_Player.BP_Player_C|GetHealthWidgetRef _asbp_player) _asbp_player)
      (Default|UpdateLivesCount (Variables|/Game/InfiniteMatrix/Blueprints/BP_Player.BP_Player_C|GetHealthWidgetRef _asbp_player)))))

(event EventTick
  (params (DeltaSeconds :type Float%20%28single-precision%29))
  (Transformation|AddActorLocalRotation (Math|Rotator|MakeRotator 0.0 0.0 (* DeltaSeconds (Variables|Default|GetRotationSpeed))) false false))

(fn ConstructionScript)